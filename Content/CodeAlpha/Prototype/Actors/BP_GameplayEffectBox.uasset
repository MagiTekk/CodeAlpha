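; BP_GameplayEffectBox is a prototype trigger actor that applies a gameplay effect to any CodeAlphaCharacter that overlaps its box.
; On begin overlap, it uses the character's Ability System Component to build a spec from OnPickupEffect and apply it to that same character.
; The construction script assigns the NiagaraVFX asset to the Niagara component when set.
; The actor has no logic to remove itself after use.
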(event OnComponentBeginOverlap(Box)
  (params (OverlappedComponent :type Primitive%20Component%20Object%20Reference) (OtherActor :type Actor%20Object%20Reference) (OtherComp :type Primitive%20Component%20Object%20Reference) (OtherBodyIndex :type Integer) (bFromSweep :type Boolean) (SweepResult :type Hit%20Result%20Structure%20%28by%20ref%29))
  (bind _ascode_alpha_character (Utilities|Casting|CastToCodeAlphaCharacter OtherActor))
  (Utilities|IsValid (Ability|GetAbilitySystemComponent _ascode_alpha_character)
    (:Is%20Valid
      (GameplayEffects|ApplyGameplayEffectSpecToSelf (Ability|GetAbilitySystemComponent _ascode_alpha_character) (GameplayEffects|MakeOutgoingSpec (Ability|GetAbilitySystemComponent _ascode_alpha_character) (Variables|CodeAlpha|Pickup|GetOnPickupEffect) 0.0 (GameplayEffects|MakeEffectContext (Ability|GetAbilitySystemComponent _ascode_alpha_character)))))))

(fn ConstructionScript
  (bind _niagaravfx (Variables|CodeAlpha|Initialization|GetNiagaraVFX)
    (:then
      (Class|NiagaraComponent|SetAsset (Variables|Default|GetNiagaraPS) _niagaravfx true))
    (:else)))